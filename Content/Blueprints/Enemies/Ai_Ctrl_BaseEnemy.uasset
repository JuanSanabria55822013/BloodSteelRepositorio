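; Base enemy AI controller that runs the possessed enemy's own behavior tree against the player.
; On possess, after a short delay, it casts to AI_BaseEnemy, starts that tree and sets player 0 as the attack target, or prints an error if no tree is valid.
; It then copies the pawn's attack and defend radii from GetIdealRangeMessage into the Blackboard.
; Helper functions switch the Blackboard's enemy-state enum between passive and attacking.
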(event `self.ReceivePossess`
  (params (PossessedPawn :type "Pawn Object Reference"))
  (`KismetSystemLibrary.Delay` 0.2)
  (bind _asai_base_enemy (cast `/Game/Blueprints/Enemies/AI/AI_BaseEnemy` PossessedPawn))
  (bind _behaviortree (`/Game/Blueprints/Enemies/AI/AI_BaseEnemy.BehaviorTree` _asai_base_enemy)
    (:`then`
      (`self.RunBehaviorTree` _behaviortree)
      (bind _output_get (set `self.AttackTarget` (`GameplayStatics.GetPlayerCharacter` 0)))
      (`self.SetStateAsAttacking` _output_get)
      (bind (_attackradius _defendradius) (message `/Game/Blueprints/Enemies/Interfaces/BPI_EnemyBase.GetIdealRange` PossessedPawn))
      (`BlackboardComponent.SetValueAsFloat` (`self.Blackboard`) (`self.Attack Radius Key Name`) _attackradius)
      (`BlackboardComponent.SetValueAsFloat` (`self.Blackboard`) (`self.Defend Radius Key Name`) _defendradius))
    (:`else`
      (`KismetSystemLibrary.PrintString` "No valid Behavier Tree in Enemy Actor"))))

(fn `SetStateAsAttacking`
  (params (EnemyActor :type "Actor Object Reference"))
  (`BlackboardComponent.SetValueAsObject` (`self.Blackboard`) (`self.AttackTarget Key Name`) EnemyActor)
  (`BlackboardComponent.SetValueAsEnum` (`self.Blackboard`) (`self.State Key Name`) (enumliteral `/Game/Blueprints/Enemies/Enums/E_EnemysStates` "NewEnumerator1")))

(fn `SetStateAsPassive`
  (`BlackboardComponent.SetValueAsEnum` (`self.Blackboard`) (`self.State Key Name`) (enumliteral `/Game/Blueprints/Enemies/Enums/E_EnemysStates` "NewEnumerator0")))

(fn `UserConstructionScript`)