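; Automated train-on-rails Blueprint that builds track along a spline and moves a train component along it.
; The construction script tiles spline mesh segments of MeshSize length with collision, clamping tangents to the segment size to follow the curve.
; Each tick advances the distance by SplineSpeed and sets the train's local position and yaw, offset -90 degrees, from the spline.
; When Loop is enabled, the distance resets to zero past the spline's end.
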(event `self.ReceiveTick`
  (params (DeltaSeconds :type "Float (single-precision)"))
  (bind _returnvalue (`SplineComponent.GetTransformAtDistanceAlongSpline` (`self.Spline`) (`self.Distance Along Spline`) "Local" false))
  (set `self.Distance Along Spline` (+ (* DeltaSeconds (`self.SplineSpeed`)) (`self.Distance Along Spline`)))
  (`SceneComponent.K2_SetRelativeTransform` (`self.Tren`) (`KismetMathLibrary.MakeTransform` (`KismetMathLibrary.MakeVector` (.x (.location _returnvalue)) (.y (.location _returnvalue)) (.z (.location _returnvalue))) (`KismetMathLibrary.MakeRotator` 0.0 0.0 (+ (.yaw (.rotation _returnvalue)) -90.0)) (`SceneComponent.RelativeScale3D` (`self.Tren`))) false false)
  (if (`self.Loop?`)
    (if (> (`self.Distance Along Spline`) (`SplineComponent.GetSplineLength` (`self.Spline`)))
      (set `self.Distance Along Spline` 0.0))))

(fn `UserConstructionScript`
  (bind _spline (`self.Spline`))
  (bind _meshsize (`self.MeshSize`))
  (for _index (range (+ (`KismetMathLibrary.FTrunc` (/ (`SplineComponent.GetSplineLength` (`self.Spline`)) (`self.MeshSize`))) 1))
    (bind _returnvalue (`AddComponent|NODE_AddSplineMeshComponent-0`))
    (bind _returnvalue_2 (* _index _meshsize))
    (bind _returnvalue_3 (+ _returnvalue_2 _meshsize))
    (`SplineMeshComponent.SetStartAndEnd` _returnvalue (`SplineComponent.GetLocationAtDistanceAlongSpline` _spline _returnvalue_2 "Local") (`KismetMathLibrary.ClampVectorSize` (`SplineComponent.GetTangentAtDistanceAlongSpline` _spline _returnvalue_2 "Local") 0.0 _meshsize) (`SplineComponent.GetLocationAtDistanceAlongSpline` _spline _returnvalue_3 "Local") (`KismetMathLibrary.ClampVectorSize` (`SplineComponent.GetTangentAtDistanceAlongSpline` _spline _returnvalue_3 "Local") 0.0 _meshsize) true)
    (`PrimitiveComponent.SetCollisionEnabled` _returnvalue "QueryAndPhysics")
    (`StaticMeshComponent.SetStaticMesh` _returnvalue (`self.mesh`))))