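; Interactive button actor that toggles a spawned object, creating it or removing it on the IA_Interact input.
; Each press plays the button animation, then either destroys the existing object or spawns ObjetoSpawn at the SpawnPoint actor's transform.
; The ObjetoCreado flag tracks state, with an IsValid check that respawns the object if it is no longer valid.
; The trailing delays lead to nothing, so they do not throttle input.
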(event `EnhancedInput|/Game/FirstPerson/Input/Actions/IA_Interact`
  (params (ActionValue :type Boolean) (ElapsedSeconds :type "Float (double-precision)") (TriggeredSeconds :type "Float (double-precision)") (InputAction :type "InputAction Object Reference" :default "/Game/FirstPerson/Input/Actions/IA_Interact.IA_Interact"))
  (:`Started`
    (`SkeletalMeshComponent.PlayAnimation` (`self.Boton`) "/Game/Models/Debugg/Boton/AnimM_Boton.AnimM_Boton" false)
    (if (`self.Objeto Creado`)
      (`/Engine/EditorBlueprintResources/StandardMacros.IsValid` (`self.Objeto`)
        (:`Is Valid`
          (`self.K2_DestroyActor` (stale _returnvalue))
          (set `self.Objeto Creado` false)
          (`KismetSystemLibrary.Delay` 0.2))
        (:`Is Not Valid`
          (set `self.Objeto Creado` false)
          (bind _returnvalue (`|SpawnActorFromClass` (`self.ObjetoSpawn`) (`self.GetTransform` (`self.SpawnPoint`)) "Undefined" "MultiplyWithRoot" null null :!label _label))
          (set `self.Objeto` _returnvalue)
          (set `self.Objeto Creado` true)
          (`KismetSystemLibrary.Delay` 0.2)))
      (else
        (goto _label)))))

(fn `UserConstructionScript`)