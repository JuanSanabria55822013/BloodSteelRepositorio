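; Overlap trigger actor that activates the tutorial through the player controller.
; On BeginPlay it casts player controller 0 to BP_PlayerControllerBase and caches it.
; The first overlap by an actor not equal to AsPlayer calls ActivarTutorial on that controller, with a DoOnce preventing repeats.
; AsPlayer is never assigned in these graphs.
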(event `self.ReceiveBeginPlay`
  (bind _asbp_player_controller_base (cast `/Game/Blueprints/Config/PlayerController/BP_PlayerControllerBase` (`GameplayStatics.GetPlayerController` 0)))
  (set `self.PlayerController` _asbp_player_controller_base))

(event `self.ReceiveActorBeginOverlap`
  (params (OtherActor :type "Actor Object Reference"))
  (if (not (== OtherActor (`self.AsPlayer`)))
    (`/Engine/EditorBlueprintResources/StandardMacros.DoOnce` false
      (:`Completed`
        (`/Game/Blueprints/Config/PlayerController/BP_PlayerControllerBase.Activar Tutorial` (`self.PlayerController`))))))

(fn `UserConstructionScript`
  (`parent.UserConstructionScript`))