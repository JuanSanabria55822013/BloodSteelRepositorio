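; BP_Trap is an electric trap that damages the player for as long as they overlap it.
; On begin overlap with the stored player reference, it applies damage, plays an electrocution sound and triggers the electricity effect on the player's damage widget.
; A one-second Delay loops back to recheck the overlap, producing damage ticks until the player leaves.
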(event `self.ReceiveActorBeginOverlap`
  (params (OtherActor :type "Actor Object Reference"))
  (bind _asplayer (`self.AsPlayer`))
  (if (== OtherActor _asplayer) :!label _label
    (if (`self.IsOverlappingActor` _asplayer)
      (`GameplayStatics.ApplyDamage` OtherActor (`self.Damage`) null self)
      (`GameplayStatics.PlaySound2D` "/Game/Sonidos/Personaje/Electrocutado.Electrocutado" 1.0 1.0 0.0 null null)
      (`/Game/Blueprints/Widgets/WBP_HUD/WBP_EffectDamage.ElectricidadDamage` (`/Game/FirstPerson/Blueprints/BP_FirstPersonCharacter.DamageWidget` _asplayer))
      (`KismetSystemLibrary.Delay` 1.0)
      (goto _label))))

(fn `UserConstructionScript`)