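; BP_Salud is a health pickup actor that heals the player on overlap.
; When the overlapping actor is the stored player reference and its HP is below or different from max, it plays a pickup sound, calls Heal on the player and destroys itself.
; At full health the pickup stays in the level.
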(event `self.ReceiveActorBeginOverlap`
  (params (OtherActor :type "Actor Object Reference"))
  (bind _asplayer (`self.AsPlayer`))
  (if (== OtherActor (`self.AsPlayer`))
    (if (not (== (`/Game/FirstPerson/Blueprints/BP_FirstPersonCharacter.HP` _asplayer) (`/Game/FirstPerson/Blueprints/BP_FirstPersonCharacter.MaxHealth` _asplayer)))
      (`GameplayStatics.PlaySound2D` "/Game/Sonidos/Personaje/recoger.recoger" 1.0 1.0 0.0 null null)
      (`/Game/FirstPerson/Blueprints/BP_FirstPersonCharacter.Heal` _asplayer (`self.Heal`))
      (`self.K2_DestroyActor`))))

(fn `UserConstructionScript`)