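; Shotgun (Escopeta) ammo pickup that reacts when the player actor overlaps it.
; On overlap it plays a 2D pickup sound, then adds 4 to the player's EscopetaComponent reserve ammo, capped at 24.
; It destroys itself even when the reserve is already full, but stays in place if the shotgun component is invalid.
; The AsPlayer reference it compares against is not assigned in these graphs.
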(event `self.ReceiveActorBeginOverlap`
  (params (OtherActor :type "Actor Object Reference"))
  (bind _escopetacomponent (`/Game/FirstPerson/Blueprints/BP_FirstPersonCharacter.EscopetaComponent` (`self.AsPlayer`)))
  (bind _reserveammo (`/Game/FirstPerson/Blueprints/LogicaArmas/BP_Weapon_ComponentEscopeta.ReserveAmmo` _escopetacomponent))
  (bind _returnvalue (+ _reserveammo 4))
  (if (== OtherActor (`self.AsPlayer`))
    (`GameplayStatics.PlaySound2D` "/Game/Sonidos/Personaje/recoger.recoger" 1.0 1.0 0.0 null null)
    (if (`KismetSystemLibrary.IsValid` _escopetacomponent)
      (if (== _reserveammo 24)
        (`self.K2_DestroyActor`)
        (else
          (if (>= _returnvalue 24)
            (set `/Game/FirstPerson/Blueprints/LogicaArmas/BP_Weapon_ComponentEscopeta.ReserveAmmo` 24 _escopetacomponent)
            (else
              (set `/Game/FirstPerson/Blueprints/LogicaArmas/BP_Weapon_ComponentEscopeta.ReserveAmmo` _returnvalue _escopetacomponent)))
          (`self.K2_DestroyActor`))))))

(fn `UserConstructionScript`)