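; BP_InteractiveActor is an interactive actor that shows an interaction prompt while the player overlaps it.
; BeginPlay caches the first-person character and testing player controller.
; Overlap begin and end toggle the actor's input, its widget and the HUD's "E" feedback text.
; The HUD calls go through PlayerControlerBase, which this graph never assigns, rather than the cached testing controller.
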(event `self.ReceiveBeginPlay`
  ;[0 0.15 0.03269 0.5] Beginplay
  (bind _asbp_first_person_character (cast `/Game/FirstPerson/Blueprints/BP_FirstPersonCharacter` (`GameplayStatics.GetPlayerPawn` 0)))
  (set `self.Player` _asbp_first_person_character)
  (bind _asbp_player_controller_testing (cast `/Game/Blueprints/Config/PlayerController/BP_PlayerControllerTesting` (`GameplayStatics.GetPlayerController` 0)))
  (set `self.PlayerControlerTesting` _asbp_player_controller_testing))

(event `self.ReceiveActorBeginOverlap`
  (params (OtherActor :type "Actor Object Reference"))
  ;[0.15 0.1375 0 0.5] BeginOverlap
  (if (== OtherActor (`self.Player`))
    (`self.EnableInput` (`GameplayStatics.GetPlayerController` 0))
    (`/Game/Blueprints/Widgets/WBP_HUD/WBP_HUB.CE_FeedbackText` (`/Game/Blueprints/Config/PlayerController/BP_PlayerControllerBase.As_HUB` (`self.PlayerControlerBase`)) "E" "Visible")
    (`SceneComponent.SetVisibility` (`self.Widget`) true false)))

(event `self.ReceiveActorEndOverlap`
  (params (OtherActor :type "Actor Object Reference"))
  ;[0 0.001713 0.15 0.5] EndOverlap
  (if (== OtherActor (`self.Player`))
    (`self.DisableInput` (`GameplayStatics.GetPlayerController` 0))
    (`/Game/Blueprints/Widgets/WBP_HUD/WBP_HUB.CE_FeedbackText` (`/Game/Blueprints/Config/PlayerController/BP_PlayerControllerBase.As_HUB` (`self.PlayerControlerBase`)) "" "Hidden")
    (`SceneComponent.SetVisibility` (`self.Widget`) false false)))

(fn `UserConstructionScript`)