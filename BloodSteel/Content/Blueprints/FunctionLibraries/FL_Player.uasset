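; FL_Player is a function library for player health and armor: healing, armor pickup and damage.
; The add functions write the clamped sum to the target actor's HP or Armadura (armor).
; TakeDamage drains armor first, carries any excess into health, and calls CEDie when health runs out.
; Every hit also plays a scaled-up Walk camera shake on player controller 0, whichever actor is damaged.
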(fn `AddArmadura`
  (params (Armature :type "Float (double-precision)") (Actor :type "/Game/FirstPerson/Blueprints/BP_FirstPersonCharacter Object Reference") (MaxArmature :type "Float (double-precision)") (AddArmature :type "Float (double-precision)"))
  (set `/Game/FirstPerson/Blueprints/BP_FirstPersonCharacter.Armadura` (`KismetMathLibrary.FClamp` (+ Armature AddArmature) 0.0 MaxArmature) Actor)
  (return))

(fn `AddHealth`
  (params (Health :type "Float (double-precision)") (MaxHealth :type "Float (double-precision)") (Heal :type "Float (double-precision)") (Actor :type "/Game/FirstPerson/Blueprints/BP_FirstPersonCharacter Object Reference"))
  (set `/Game/FirstPerson/Blueprints/BP_FirstPersonCharacter.HP` (`KismetMathLibrary.FClamp` (+ Health Heal) 0.0 MaxHealth) Actor)
  (return))

(fn `TakeDamage`
  (params (Health :type "Float (double-precision)") (Armature :type "Float (double-precision)") (Damage :type "Float (double-precision)") (Actor :type "/Game/FirstPerson/Blueprints/BP_FirstPersonCharacter Object Reference"))
  (bind _returnvalue (- Health Damage))
  (bind _returnvalue_2 (- Armature Damage))
  (bind _returnvalue_3 (+ Health _returnvalue_2))
  (if (== Armature 0.0)
    (if (<= _returnvalue 0.0)
      (set `/Game/FirstPerson/Blueprints/BP_FirstPersonCharacter.HP` 0.0 Actor :!label _label)
      (`/Game/FirstPerson/Blueprints/BP_FirstPersonCharacter.CE_Die` Actor)
      (else
        (set `/Game/FirstPerson/Blueprints/BP_FirstPersonCharacter.HP` _returnvalue Actor)))
    (elif (< _returnvalue_2 0.0)
      (set `/Game/FirstPerson/Blueprints/BP_FirstPersonCharacter.Armadura` 0.0 Actor)
      (if (<= _returnvalue_3 0.0)
        (goto _label)
        (else
          (set `/Game/FirstPerson/Blueprints/BP_FirstPersonCharacter.HP` _returnvalue_3 Actor)))
      (else
        (set `/Game/FirstPerson/Blueprints/BP_FirstPersonCharacter.Armadura` _returnvalue_2 Actor))))
  (`PlayerController.ClientStartCameraShake` :`self` (`GameplayStatics.GetPlayerController` null) :`Shake` "/Game/FirstPerson/Blueprints/CameraShakes/Walk.Walk_C" :`Scale` 5.0)
  (return))