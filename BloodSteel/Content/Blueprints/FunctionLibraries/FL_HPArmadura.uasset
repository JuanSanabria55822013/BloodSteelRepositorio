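; Blueprint function library that applies health and armor changes to the player and to the Fornax and Centinela characters.
; Each function adds a signed amount to the target's stat and clamps it at zero, with health also capped at a hardcoded maximum per character type.
; Health reaching zero calls the target's death event or function, while armor has no upper limit and triggers nothing.
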(fn `AddArmadura`
  (params (ArmaduraToAdd1 :type Integer) (Player1 :type "/Game/FirstPerson/Blueprints/BP_FirstPersonCharacter Object Reference"))
  (locals (ArmaduraToAdd :type Integer) (Player :type "/Game/FirstPerson/Blueprints/BP_FirstPersonCharacter Object Reference"))
  (set `local.ArmaduraToAdd` ArmaduraToAdd1)
  (set `local.Player` Player1)
  (if (<= (+ (`local.ArmaduraToAdd`) (`/Game/FirstPerson/Blueprints/BP_FirstPersonCharacter.Armadura` (`local.Player`))) 0)
    (set `/Game/FirstPerson/Blueprints/BP_FirstPersonCharacter.Armadura` 0 (`local.Player`))
    (else
      (set `/Game/FirstPerson/Blueprints/BP_FirstPersonCharacter.Armadura` (+ (`local.ArmaduraToAdd`) (`/Game/FirstPerson/Blueprints/BP_FirstPersonCharacter.Armadura` (`local.Player`))) (`local.Player`))))
  (return))

(fn `AddHP`
  (params (HpToAdd1 :type Integer) (Player1 :type "/Game/FirstPerson/Blueprints/BP_FirstPersonCharacter Object Reference"))
  (locals (HpToAdd :type Integer) (Player :type "/Game/FirstPerson/Blueprints/BP_FirstPersonCharacter Object Reference"))
  (set `local.HpToAdd` HpToAdd1)
  (set `local.Player` Player1)
  (if (<= (+ (`/Game/FirstPerson/Blueprints/BP_FirstPersonCharacter.HP` (`local.Player`)) (`local.HpToAdd`)) 0)
    (set `/Game/FirstPerson/Blueprints/BP_FirstPersonCharacter.HP` 0 (`local.Player`))
    (`/Game/FirstPerson/Blueprints/BP_FirstPersonCharacter.CE_Die` (`local.Player`))
    (elif (>= (+ (`/Game/FirstPerson/Blueprints/BP_FirstPersonCharacter.HP` (`local.Player`)) (`local.HpToAdd`)) 100)
      (set `/Game/FirstPerson/Blueprints/BP_FirstPersonCharacter.HP` 100 (`local.Player`))
      (else
        (set `/Game/FirstPerson/Blueprints/BP_FirstPersonCharacter.HP` (+ (`/Game/FirstPerson/Blueprints/BP_FirstPersonCharacter.HP` (`local.Player`)) (`local.HpToAdd`)) (`local.Player`)))))
  (return))

(fn `HPCentinela`
  (params (AddHp1 :type Integer) (Centinela1 :type "/Game/Blueprints/Enemies/Centinela/AI_Centinela Object Reference"))
  (locals (Centinela :type "/Game/Blueprints/Enemies/Centinela/AI_Centinela Object Reference") (AddHp :type Integer))
  (set `local.AddHp` AddHp1)
  (bind _output_get (set `local.Centinela` Centinela1))
  (if (<= (+ (`/Game/Blueprints/Enemies/Centinela/AI_Centinela.HP` _output_get) (`local.AddHp`)) 0)
    (set `/Game/Blueprints/Enemies/Centinela/AI_Centinela.HP` 0 (`local.Centinela`))
    (`/Game/Blueprints/Enemies/Centinela/AI_Centinela.Die` (`local.Centinela`))
    (elif (>= (+ (`/Game/Blueprints/Enemies/Centinela/AI_Centinela.HP` (`local.Centinela`)) (`local.AddHp`)) 25)
      (set `/Game/Blueprints/Enemies/Centinela/AI_Centinela.HP` 25 (`local.Centinela`))
      (else
        (set `/Game/Blueprints/Enemies/Centinela/AI_Centinela.HP` (+ (`/Game/Blueprints/Enemies/Centinela/AI_Centinela.HP` (`local.Centinela`)) (`local.AddHp`)) (`local.Centinela`)))))
  (return))

(fn `HPFornax`
  (params (AddHp1 :type Integer) (Fonax1 :type "/Game/Blueprints/Enemies/Fornax/AI_Fornax Object Reference"))
  (locals (Fonax :type "/Game/Blueprints/Enemies/Fornax/AI_Fornax Object Reference") (AddHp :type Integer))
  (set `local.AddHp` AddHp1)
  (set `local.Fonax` Fonax1)
  (if (<= (+ (`/Game/Blueprints/Enemies/Fornax/AI_Fornax.HP` (`local.Fonax`)) (`local.AddHp`)) 0)
    (set `/Game/Blueprints/Enemies/Fornax/AI_Fornax.HP` 0 (`local.Fonax`))
    (`/Game/Blueprints/Enemies/Fornax/AI_Fornax.Die` (`local.Fonax`))
    (elif (>= (+ (`/Game/Blueprints/Enemies/Fornax/AI_Fornax.HP` (`local.Fonax`)) (`local.AddHp`)) 100)
      (set `/Game/Blueprints/Enemies/Fornax/AI_Fornax.HP` 100 (`local.Fonax`))
      (else
        (set `/Game/Blueprints/Enemies/Fornax/AI_Fornax.HP` (+ (`/Game/Blueprints/Enemies/Fornax/AI_Fornax.HP` (`local.Fonax`)) (`local.AddHp`)) (`local.Fonax`)))))
  (return))