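; Testing player controller that adds debug cheats to the first-person game alongside the usual HUD and pause menu.
; On BeginPlay it creates the widgets; IA_Pause swaps HUD and pause menu, and Tab toggles the testing overlay.
; Z, X and C toggle immortality, infinite ammo and half-speed time dilation, while numpad keys forward to the character and overlay.
; Debugg exposes those flags plus fixed stat increments; CheckPoint is an empty stub.
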(event `self.ReceiveBeginPlay`
  (bind _returnvalue (`GameplayStatics.GetPlayerController` 0))
  (bind _asbp_first_person_character (cast `/Game/FirstPerson/Blueprints/BP_FirstPersonCharacter` (`GameplayStatics.GetPlayerPawn` 0)))
  (`/Engine/EditorBlueprintResources/StandardMacros.IsValid` _asbp_first_person_character
    (:`Is Valid`
      (set `self.Jugador` _asbp_first_person_character)
      (`WidgetBlueprintLibrary.SetInputMode_GameOnly` _returnvalue)
      (set `PlayerController.bShowMouseCursor` false _returnvalue)
      (`GameplayStatics.SetGamePaused` false)
      (bind _returnvalue_2 (`|GenericCreateObject` "/Game/Blueprints/Widgets/WBP_HUD/WBP_HUB.WBP_HUB_C"))
      (bind _output_get (set `self.As_HUB` _returnvalue_2))
      (`UserWidget.AddToViewport` _output_get 0)
      (bind _returnvalue_3 (`|GenericCreateObject` "/Game/Blueprints/Widgets/WBP_HUD/WBP_Testing.WBP_Testing_C"))
      (bind _output_get_2 (set `self.As_Testing` _returnvalue_3))
      (set `self.AsTesting` true)
      (`UserWidget.AddToViewport` _output_get_2 0)
      (bind _returnvalue_4 (`|GenericCreateObject` "/Game/Blueprints/Widgets/WBP_Pantallas/WBP_PauseMenu.WBP_PauseMenu_C"))
      (set `self.As_PauseMenu` _returnvalue_4))))

(event `EnhancedInput|/Game/FirstPerson/Input/Actions/IA_Pause`
  (params (ActionValue :type Boolean) (ElapsedSeconds :type "Float (double-precision)") (TriggeredSeconds :type "Float (double-precision)") (InputAction :type "InputAction Object Reference" :default "/Game/FirstPerson/Input/Actions/IA_Pause.IA_Pause"))
  (:`Started`
    (`self.F_Pause`)))

(event `Key|Tab`
  (params (Key :type "Key Structure"))
  (:`Pressed`
    (if (`self.AsTesting`)
      (`Widget.RemoveFromParent` (`self.As_Testing`))
      (set `self.AsTesting` false)
      (else
        (`UserWidget.AddToViewport` (`self.As_Testing`) 0)
        (set `self.AsTesting` true)))))

(event `Key|Z`
  (params (Key :type "Key Structure"))
  (:`Pressed`
    (set `self.Inmortal` (not (`self.Inmortal`)))))

(event `Key|X`
  (params (Key :type "Key Structure"))
  (:`Pressed`
    (set `self.InfiniteAmmo` (not (`self.InfiniteAmmo`)))))

(event `Key|C`
  (params (Key :type "Key Structure"))
  (:`Pressed`
    (`/Engine/EditorBlueprintResources/StandardMacros.FlipFlop`
      (:`A`
        (`GameplayStatics.SetGlobalTimeDilation` 0.5)
        (set `self.SlowMo` true))
      (:`B`
        (`GameplayStatics.SetGlobalTimeDilation` 1.0)
        (set `self.SlowMo` false)))))

(event `Key|NumPadOne`
  (params (Key :type "Key Structure"))
  (:`Pressed`
    (`/Game/FirstPerson/Blueprints/BP_FirstPersonCharacter.Num1` (`self.Jugador`))
    (`/Game/Blueprints/Widgets/WBP_HUD/WBP_Testing.ClickNum1` (`self.As_Testing`))))

(event `Key|NumPadThree`
  (params (Key :type "Key Structure"))
  (:`Pressed`
    (`/Game/FirstPerson/Blueprints/BP_FirstPersonCharacter.Num3` (`self.Jugador`))
    (`/Game/Blueprints/Widgets/WBP_HUD/WBP_Testing.ClickNum3` (`self.As_Testing`))))

(event `Key|NumPadFour`
  (params (Key :type "Key Structure"))
  (:`Pressed`
    (`/Game/FirstPerson/Blueprints/BP_FirstPersonCharacter.Num4` (`self.Jugador`))
    (`/Game/Blueprints/Widgets/WBP_HUD/WBP_Testing.ClickNum4` (`self.As_Testing`))))

(event `Key|NumPadSix`
  (params (Key :type "Key Structure"))
  (:`Pressed`
    (`/Game/FirstPerson/Blueprints/BP_FirstPersonCharacter.Num 6` (`self.Jugador`))
    (`/Game/Blueprints/Widgets/WBP_HUD/WBP_Testing.ClickNum6` (`self.As_Testing`))))

(event `Key|NumPadSeven`
  (params (Key :type "Key Structure"))
  (:`Pressed`
    (`/Game/FirstPerson/Blueprints/BP_FirstPersonCharacter.Num 7` (`self.Jugador`))
    (`/Game/Blueprints/Widgets/WBP_HUD/WBP_Testing.ClickNum7` (`self.As_Testing`))))

(event `Key|NumPadNine`
  (params (Key :type "Key Structure"))
  (:`Pressed`
    (`/Game/FirstPerson/Blueprints/BP_FirstPersonCharacter.Num 9` (`self.Jugador`))
    (`/Game/Blueprints/Widgets/WBP_HUD/WBP_Testing.ClickNum9` (`self.As_Testing`))))

(event `Key|NumPadEight`
  (params (Key :type "Key Structure"))
  (:`Pressed`
    (`/Game/FirstPerson/Blueprints/BP_FirstPersonCharacter.Num 8` (`self.Jugador`))
    (`/Game/Blueprints/Widgets/WBP_HUD/WBP_Testing.ClickNum8` (`self.As_Testing`))))

(event `Key|NumPadTwo`
  (params (Key :type "Key Structure"))
  (:`Pressed`
    (`/Game/FirstPerson/Blueprints/BP_FirstPersonCharacter.Num 2` (`self.Jugador`))
    (`/Game/Blueprints/Widgets/WBP_HUD/WBP_Testing.ClickNum2` (`self.As_Testing`))))

(fn `CheckPoint`)

(fn `Debugg`
  (returns (Inmortal :type Boolean) (InfiniteAmmo :type Boolean) (SlowMo :type Boolean) (MasVida :type "Float (double-precision)") (MenosVida :type "Float (double-precision)") (MasVelocidad :type "Float (double-precision)") (MenosVelocidad :type "Float (double-precision)") (MasArmadura :type "Float (double-precision)") (MenosArmadura :type "Float (double-precision)") (`MasDaño` :type "Float (double-precision)") (`MenosDaño` :type "Float (double-precision)") (MasAltura :type "Float (double-precision)") (MenosAltura :type "Float (double-precision)"))
  (return (`self.Inmortal`) (`self.InfiniteAmmo`) (`self.SlowMo`) 10.0 -10.0 100.0 -100.0 10.0 -10.0 5.0 -5.0 50.0 -50.0))

(fn `F_Pause`
  (bind _returnvalue (`GameplayStatics.GetPlayerController` 0))
  (bind _returnvalue_2 (`GameplayStatics.GetPlayerController` 0))
  (if (`GameplayStatics.IsGamePaused`)
    (`/Game/Blueprints/Widgets/WBP_Pantallas/WBP_PauseMenu.ResetMenu` (`self.As_PauseMenu`))
    (`Widget.RemoveFromParent` (`self.As_PauseMenu`))
    (if (`KismetSystemLibrary.IsValid` _returnvalue)
      (`WidgetBlueprintLibrary.SetInputMode_GameOnly` _returnvalue)
      (set `PlayerController.bShowMouseCursor` false _returnvalue)
      (`UserWidget.AddToViewport` (`self.As_HUB`) 0)
      (`GameplayStatics.SetGamePaused` false))
    (else
      (`Widget.RemoveFromParent` (`self.As_HUB`))
      (`UserWidget.AddToViewport` (`self.As_PauseMenu`) 0)
      (if (`KismetSystemLibrary.IsValid` _returnvalue_2)
        (`WidgetBlueprintLibrary.SetInputMode_GameAndUIEx` _returnvalue_2 null)
        (set `PlayerController.bShowMouseCursor` true _returnvalue_2)
        (`GameplayStatics.SetGamePaused` true)))))

(fn `UserConstructionScript`)