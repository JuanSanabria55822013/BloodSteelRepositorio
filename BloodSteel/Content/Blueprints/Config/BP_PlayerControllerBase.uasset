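; Base player controller that sets up the HUB widget and pause menu and handles pausing the game.
; BeginPlay sets game-only input, hides the cursor, unpauses, shows WBP_HUB and pre-creates WBP_PauseMenu.
; The IA_Pause input calls FPause, which toggles pause by swapping the two widgets, input mode and cursor visibility, resetting the menu on resume.
; The CheckPoint function is an empty stub.
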(event `self.ReceiveBeginPlay`
  (bind _returnvalue (`GameplayStatics.GetPlayerController` 0))
  (`WidgetBlueprintLibrary.SetInputMode_GameOnly` _returnvalue)
  (set `PlayerController.bShowMouseCursor` false _returnvalue)
  (`GameplayStatics.SetGamePaused` false)
  (bind _returnvalue_2 (`|GenericCreateObject` "/Game/Blueprints/Widgets/WBP_HUD/WBP_HUB.WBP_HUB_C"))
  (bind _output_get (set `self.As_HUB` _returnvalue_2))
  (`UserWidget.AddToViewport` _output_get 0)
  (bind _returnvalue_3 (`|GenericCreateObject` "/Game/Blueprints/Widgets/WBP_Pantallas/WBP_PauseMenu.WBP_PauseMenu_C"))
  (set `self.As_PauseMenu` _returnvalue_3))

(event `Key|Z`
  (params (Key :type "Key Structure")))

(event `EnhancedInput|/Game/FirstPerson/Input/Actions/IA_Pause`
  (params (ActionValue :type Boolean) (ElapsedSeconds :type "Float (double-precision)") (TriggeredSeconds :type "Float (double-precision)") (InputAction :type "InputAction Object Reference" :default "/Game/FirstPerson/Input/Actions/IA_Pause.IA_Pause"))
  (:`Started`
    (`self.F_Pause`)))

(fn `CheckPoint`)

(fn `F_Pause`
  (bind _returnvalue (`GameplayStatics.GetPlayerController` 0))
  (bind _returnvalue_2 (`GameplayStatics.GetPlayerController` 0))
  (if (`GameplayStatics.IsGamePaused`)
    (`/Game/Blueprints/Widgets/WBP_Pantallas/WBP_PauseMenu.ResetMenu` (`self.As_PauseMenu`))
    (`Widget.RemoveFromParent` (`self.As_PauseMenu`))
    (if (`KismetSystemLibrary.IsValid` _returnvalue)
      (`WidgetBlueprintLibrary.SetInputMode_GameOnly` _returnvalue)
      (set `PlayerController.bShowMouseCursor` false _returnvalue)
      (`UserWidget.AddToViewport` (`self.As_HUB`) 0)
      (`GameplayStatics.SetGamePaused` false))
    (else
      (`Widget.RemoveFromParent` (`self.As_HUB`))
      (`UserWidget.AddToViewport` (`self.As_PauseMenu`) 0)
      (if (`KismetSystemLibrary.IsValid` _returnvalue_2)
        (`WidgetBlueprintLibrary.SetInputMode_GameAndUIEx` _returnvalue_2 null)
        (set `PlayerController.bShowMouseCursor` true _returnvalue_2)
        (`GameplayStatics.SetGamePaused` true)))))

(fn `UserConstructionScript`)