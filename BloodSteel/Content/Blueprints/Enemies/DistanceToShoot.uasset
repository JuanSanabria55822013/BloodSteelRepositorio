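; Behavior tree decorator for Fornax enemy AI that checks whether the blackboard target is within shooting range.
; It returns false if AIRef is already set, otherwise it casts the owner to AI_Controller_Fornax and caches it there.
; It then compares the distance between the controlled pawn and the TargetToFollow actor against DistanceToShoot, failing when the target is invalid.
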(fn `PerformConditionCheck`
  (params (OwnerActor :type "Actor Object Reference"))
  (returns (ReturnValue :type Boolean))
  (bind _returnvalue (`BTFunctionLibrary.GetBlackboardValueAsActor` (`self.TargetToFollow`)))
  (if (!= (`self.AI_Ref`) null)
    (return false)
    (else
      (bind _asai_controller_fornax (cast `/Game/Blueprints/Enemies/AI_Controller_Fornax` OwnerActor))
      (bind _output_get (set `self.AI_Ref` _asai_controller_fornax))
      (if (`KismetSystemLibrary.IsValid` _returnvalue)
        (return (<= (`KismetMathLibrary.Vector_Distance` (`Actor.K2_GetActorLocation` (`Controller.K2_GetPawn` _output_get)) (`Actor.K2_GetActorLocation` _returnvalue)) (`self.DistanceToShoot`)))
        (else
          (return false))))))