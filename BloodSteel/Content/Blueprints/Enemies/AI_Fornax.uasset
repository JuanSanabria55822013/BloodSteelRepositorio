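; Fornax enemy AI that shoots projectiles at the first-person player and can be destroyed.
; StartDisparoLoop and StopDisparoLoop toggle a looping timer on IA_Fire, which spawns BP_DisparoFornax from a mesh socket, aimed at the cached player pawn.
; Die, at zero HP, plays explosion effects, stops the firing timer, randomly drops a BP_Salud pickup and destroys the actor.
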(event `Die`
  (bind _returnvalue (`self.K2_GetActorLocation` self))
  (if (== (`self.HP`) 0)
    (`GameplayStatics.SpawnEmitterAtLocation` "/Game/StarterContent/Particles/P_Explosion.P_Explosion" _returnvalue)
    (`GameplayStatics.PlaySoundAtLocation` "/Game/StarterContent/Audio/Explosion02.Explosion02" (0.0 0.0 0.0) (struct) 1.0 1.0 0.0 null null null null)
    (`self.StopDisparoLoop`)
    (if (< (`KismetMathLibrary.RandomFloatInRange` 0.0 1.0) 0.5)
      (`|SpawnActorFromClass` "/Game/Blueprints/OverlappingActors/BP_Salud.BP_Salud_C" (`KismetMathLibrary.MakeTransform` _returnvalue (`KismetMathLibrary.Conv_VectorToRotator` _returnvalue)) "Undefined" "MultiplyWithRoot" null null))
    (`self.K2_DestroyActor`)))

(event `IA_Fire`
  (bind _returnvalue (`SceneComponent.GetSocketLocation` (`self.Mesh`) "FornaxFireSokect"))
  (bind _returnvalue_2 (+ _returnvalue (`SceneComponent.GetForwardVector` (`self.Mesh`))))
  (if (not (!= (`self.Player`) null))
    (bind _asbp_first_person_character (cast `/Game/FirstPerson/Blueprints/BP_FirstPersonCharacter` (`GameplayStatics.GetPlayerPawn` 0)))
    (set `self.Player` _asbp_first_person_character))
  (`|SpawnActorFromClass` "/Game/Blueprints/Enemies/BP_DisparoFornax.BP_DisparoFornax_C" (`KismetMathLibrary.MakeTransform` _returnvalue_2 (`KismetMathLibrary.FindLookAtRotation` _returnvalue (`self.K2_GetActorLocation` (`self.Player`)))) "Undefined" "MultiplyWithRoot" null 25000.0 null)
  (`GameplayStatics.PlaySoundAtLocation` "/Game/StarterContent/Audio/Explosion_Cue.Explosion_Cue" _returnvalue_2 (struct) 1.0 1.0 0.0 null null null null))

(event `StartDisparoLoop`
  (`KismetSystemLibrary.K2_SetTimer` null "IA_Fire" 1.5 true))

(event `StopDisparoLoop`
  (`KismetSystemLibrary.K2_ClearTimer` null "IA_Fire"))

(fn `UserConstructionScript`)