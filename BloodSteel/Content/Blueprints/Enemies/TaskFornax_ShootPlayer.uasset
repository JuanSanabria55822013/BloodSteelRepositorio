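; Behavior tree task that makes the Fornax enemy start shooting when it has a target to follow.
; On execute it casts and caches the Fornax AI controller and its pawn, then validates the pawn and the TargetToFollow blackboard actor.
; It calls StartDisparoLoop on the pawn and immediately finishes with success.
; Failed casts or validity checks leave the task without a FinishExecute call.
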(event `self.ReceiveExecute`
  (params (OwnerActor :type "Actor Object Reference"))
  (if (not (!= (`self.AI_Ref`) null))
    (bind _asai_controller_fornax (cast `/Game/Blueprints/Enemies/AI_Controller_Fornax` OwnerActor))
    (set `self.AI_Ref` _asai_controller_fornax))
  (if (`KismetSystemLibrary.IsValid` (`Controller.K2_GetPawn` (`self.AI_Ref`)))
    (if (`KismetSystemLibrary.IsValid` (`BTFunctionLibrary.GetBlackboardValueAsActor` (`self.TargetToFollow`)))
      (if (not (!= (`self.AI_Enemi`) null))
        (bind _asai_fornax (cast `/Game/Blueprints/Enemies/AI_Fornax` (`Controller.K2_GetPawn` (`self.AI_Ref`))))
        (set `self.AI_Enemi` _asai_fornax))
      (`/Game/Blueprints/Enemies/AI_Fornax.StartDisparoLoop` (`self.AI_Enemi`))
      (`self.FinishExecute` true))))