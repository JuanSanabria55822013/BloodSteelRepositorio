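; Behavior tree tick logic that finds and tracks a visible target for the Fornax AI enemy.
; Each tick it sphere-traces for nearby objects, then line-traces on the Camera channel to each hit, ignoring all Fornax actors.
; A visible hit fills the blackboard target, location and distance, with CanShoot true when that distance is near DesideredDistance.
; Blocked hits clear TargetToFollow, and the search stops at the first valid visible target.
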(event `self.ReceiveTickAI`
  (params (OwnerController :type "AIController Object Reference") (ControlledPawn :type "Pawn Object Reference") (DeltaSeconds :type "Float (single-precision)"))
  (bind _distancetotarget (`self.DistanceToTarget`))
  (bind _canshoot (`self.CanShoot`))
  (if (not (!= (`self.AlCtrlRef`) null))
    (bind _asai_controller_fornax (cast `/Game/Blueprints/Enemies/AI_Controller_Fornax` OwnerController))
    (set `self.AlCtrlRef` _asai_controller_fornax))
  (set `self.MyLocation` (`Actor.K2_GetActorLocation` (`Controller.K2_GetPawn` (`self.AlCtrlRef`))))
  (bind _outactors (`GameplayStatics.GetAllActorsOfClass` "/Game/Blueprints/Enemies/AI_Fornax.AI_Fornax_C"))
  (bind _outhits (`KismetSystemLibrary.SphereTraceMultiForObjects` (`self.MyLocation`) (+ (`self.MyLocation`) (0.0 0.0 15.0)) 1500.0 (`self.DesiredObjectTypes`) false _outactors))
  (for _array_element _outhits
    (bind (_bblockinghit _binitialoverlap _time _distance _location _impactpoint _normal _impactnormal _physmat _hitactor) (`GameplayStatics.BreakHitResult` _array_element))
    (bind _outhit (`KismetSystemLibrary.LineTraceSingle` (`self.MyLocation`) (`Actor.K2_GetActorLocation` _hitactor) "TraceTypeQuery2" false _outactors))
    (bind (_bblockinghit_2 _binitialoverlap_2 _time_2 _distance_2 _location_2 _impactpoint_2 _normal_2 _impactnormal_2 _physmat_2 _hitactor_2) (`GameplayStatics.BreakHitResult` _outhit))
    (if (== _hitactor_2 _hitactor)
      (`BTFunctionLibrary.SetBlackboardValueAsObject` (`self.TargetToFollow`) _hitactor_2)
      (`BTFunctionLibrary.SetBlackboardValueAsVector` (`self.TargetLocation`) (`Actor.K2_GetActorLocation` _hitactor_2))
      (bind _output_get (set `self.TargetActor` (`BTFunctionLibrary.GetBlackboardValueAsActor` (`self.TargetToFollow`))))
      (if (`KismetSystemLibrary.IsValid` _output_get)
        (bind _output_get_2 (set `self.Distance` (`KismetMathLibrary.VSize` (- (`self.MyLocation`) (`Actor.K2_GetActorLocation` (`self.TargetActor`))))))
        (`BTFunctionLibrary.SetBlackboardValueAsFloat` _distancetotarget _output_get_2)
        (if (< (`KismetMathLibrary.Abs` (- (`BTFunctionLibrary.GetBlackboardValueAsFloat` _distancetotarget) (`BTFunctionLibrary.GetBlackboardValueAsFloat` (`self.DesideredDistance`)))) 800.0)
          (`BTFunctionLibrary.SetBlackboardValueAsBool` _canshoot true)
          (break)
          (else
            (`BTFunctionLibrary.SetBlackboardValueAsBool` _canshoot)
            (break))))
      (else
        (`BTFunctionLibrary.SetBlackboardValueAsObject` (`self.TargetToFollow`))))))