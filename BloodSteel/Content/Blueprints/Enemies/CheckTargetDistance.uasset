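; Behavior tree decorator for Fornax enemy AI that checks whether the followed target is farther away than a set Distance.
; It casts the owner to AI_Controller_Fornax, caches it, and reads the target actor from the TargetToFollow blackboard key.
; It passes when the distance between target and controlled pawn exceeds Distance, and fails if the cast or target is invalid.
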(fn `PerformConditionCheck`
  (params (OwnerActor :type "Actor Object Reference"))
  (returns (ReturnValue :type Boolean))
  (bind _returnvalue (`BTFunctionLibrary.GetBlackboardValueAsActor` (`self.TargetToFollow`)))
  (bind _asai_controller_fornax (cast `/Game/Blueprints/Enemies/AI_Controller_Fornax` OwnerActor)
    (:`then`
      (set `self.AICtrlRef` _asai_controller_fornax)
      (if (`KismetSystemLibrary.IsValid` _returnvalue)
        (return (> (`KismetMathLibrary.Vector_Distance` (`Actor.K2_GetActorLocation` _returnvalue) (`Actor.K2_GetActorLocation` (`Controller.K2_GetPawn` (`self.AICtrlRef`)))) (`self.Distance`)))
        (else
          (return false))))
    (:`CastFailed`
      (return false))))