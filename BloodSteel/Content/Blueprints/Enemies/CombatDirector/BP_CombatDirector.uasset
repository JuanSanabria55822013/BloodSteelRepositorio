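; Combat director actor that runs a staged combat scenario, starting when the player first overlaps it and broadcasting scenario and stage events.
; After a short delay on BeginPlay it collects overlapping AI_BaseEnemy actors and binds their death events, with AddEnemy registering more.
; Stages come from a map and either set a timer or complete once living enemies drop to a body-count threshold.
; Completing a stage advances to the next, or finishes the scenario.
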(event `self.ReceiveActorBeginOverlap`
  (params (OtherActor :type "Actor Object Reference"))
  (if (== OtherActor (`GameplayStatics.GetPlayerCharacter` 0))
    (`/Engine/EditorBlueprintResources/StandardMacros.DoOnce` false
      (:`Completed`
        (`self.StartStage`)
        (`self.OnCombatScenaryStarted`)))))

(event `self.ReceiveBeginPlay`
  (`KismetSystemLibrary.Delay` 0.2)
  (bind _output_get (set `self.EnemyActors` (`self.GetOverlappingActors` "/Game/Blueprints/Enemies/AI/AI_BaseEnemy.AI_BaseEnemy_C")))
  (for _array_element _output_get
    (bind _asai_base_enemy (cast `/Game/Blueprints/Enemies/AI/AI_BaseEnemy` _array_element))
    (add `/Game/Blueprints/Enemies/AI/AI_BaseEnemy.Dead` _asai_base_enemy (`|CreateDelegate` :!event `OnEnemyDead`))))

(event `OnEnemyDead`
  (params (Enemy :type "/Game/Blueprints/Enemies/AI/AI_BaseEnemy Object Reference"))
  (bind _enemyactors (`self.EnemyActors`))
  (`KismetArrayLibrary.Array_Remove` _enemyactors (`KismetArrayLibrary.Array_Find` _enemyactors Enemy))
  (if (<= (`KismetArrayLibrary.Array_Length` (`self.EnemyActors`)) (`self.BodyCountRemaining`))
    (`self.CompleteStage`)))

(event `CombatScenaryFinished`
  (`self.OnCombatScenaryFinished`))

(fn `ActivateEnemies`
  (for _array_element (`self.EnemyActors`)
    (message `/Game/Blueprints/Enemies/Interfaces/BPI_Combat.InitialiseCombat` _array_element)))

(fn `Add Enemy`
  (params (Enemy :type "/Game/Blueprints/Enemies/AI/AI_BaseEnemy Object Reference"))
  (`KismetArrayLibrary.Array_AddUnique` (`self.EnemyActors`) Enemy)
  (add `/Game/Blueprints/Enemies/AI/AI_BaseEnemy.Dead` Enemy (`|CreateDelegate` :!event `OnEnemyDead`)))

(fn `CompleteStage`
  (`KismetSystemLibrary.PrintString` "Complete Stage")
  (`self.OnCombatStageEnded` (`self.CurrentStage`))
  (bind _result (`/Engine/EditorBlueprintResources/StandardMacros.IncrementInt` (`self.CurrentStage`))
    (:`  `
      (if (`.ReturnValue` (`BlueprintMapLibrary.Map_Find` (`self.Stages`) _result))
        (`self.StartStage`)
        (else
          (`self.CombatScenaryFinished`))))))

(fn `StartStage`
  (bind _value (`BlueprintMapLibrary.Map_Find` (`self.Stages`) (`self.CurrentStage`)))
  (`KismetSystemLibrary.PrintString` "StartStage")
  (`self.OnCombatStageStarted` (`self.CurrentStage`))
  (switch `/Game/Blueprints/Enemies/CombatDirector/Enum_CombatStages` (break `/Game/Blueprints/Enemies/CombatDirector/FCombatStage` _value)
    (:`NewEnumerator0`
      (`KismetSystemLibrary.K2_SetTimerDelegate` (`|CreateDelegate` :!event `CompleteStage`) (`.Value_5_D465C1AC440E936CB800EC99F65C0D32` (break `/Game/Blueprints/Enemies/CombatDirector/FCombatStage` _value))))
    (:`NewEnumerator1`
      (set `self.BodyCountRemaining` (`.Value_5_D465C1AC440E936CB800EC99F65C0D32` (break `/Game/Blueprints/Enemies/CombatDirector/FCombatStage` _value))))))

(fn `UserConstructionScript`)