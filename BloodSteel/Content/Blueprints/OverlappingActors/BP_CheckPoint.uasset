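; Checkpoint actor that saves the player's state to the game instance when the player overlaps it.
; A DoOnce limits the save to the first overlap.
; It copies health, armor, dash and jump limits, weapon ownership and active weapon slot, clears the Inicio flag and records itself as the last checkpoint.
; The player and game instance references it uses are not assigned in these graphs.
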(event `self.ReceiveActorBeginOverlap`
  (params (OtherActor :type "Actor Object Reference"))
  (if (== OtherActor (`self.AsPlayer`))
    (`/Engine/EditorBlueprintResources/StandardMacros.DoOnce` false
      (:`Completed`
        (set `/Game/Blueprints/Config/BP_MyGameInstance.LastHP` (`/Game/FirstPerson/Blueprints/BP_FirstPersonCharacter.HP` (`self.AsPlayer`)) (`self.AsGameInstance`))
        (set `/Game/Blueprints/Config/BP_MyGameInstance.LastArmadura` (`/Game/FirstPerson/Blueprints/BP_FirstPersonCharacter.Armadura` (`self.AsPlayer`)) (`self.AsGameInstance`))
        (set `/Game/Blueprints/Config/BP_MyGameInstance.LastMaxCountDash` (`/Game/FirstPerson/Blueprints/BP_FirstPersonCharacter.MaxDashCount` (`self.AsPlayer`)) (`self.AsGameInstance`))
        (set `/Game/Blueprints/Config/BP_MyGameInstance.LastMaxCountJump` (`Character.JumpMaxCount` (`self.AsPlayer`)) (`self.AsGameInstance`))
        (set `/Game/Blueprints/Config/BP_MyGameInstance.HasRifle` (`/Game/FirstPerson/Blueprints/BP_FirstPersonCharacter.bHasRifle` (`self.AsPlayer`)) (`self.AsGameInstance`))
        (set `/Game/Blueprints/Config/BP_MyGameInstance.HasEscopeta` (`/Game/FirstPerson/Blueprints/BP_FirstPersonCharacter.bHasEscopeta` (`self.AsPlayer`)) (`self.AsGameInstance`))
        (set `/Game/Blueprints/Config/BP_MyGameInstance.Inicio` false (`self.AsGameInstance`))
        (set `/Game/Blueprints/Config/BP_MyGameInstance.CurrentWeapon` (`/Game/FirstPerson/Blueprints/BP_FirstPersonCharacter.ActiveWeaponSlot` (`self.AsPlayer`)) (`self.AsGameInstance`))
        (set `/Game/Blueprints/Config/BP_MyGameInstance.LastCheckpoint` (`|ConvertAsset` self) (`self.AsGameInstance`))))))

(fn `UserConstructionScript`)