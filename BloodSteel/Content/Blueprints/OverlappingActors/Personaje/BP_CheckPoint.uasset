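; BP_CheckPoint is a checkpoint actor that saves the player's progress to the game instance when the player overlaps it.
; A DoOnce limits the save to the first valid overlap.
; It writes health, armor, dash, jump and weapon ownership state plus a reference to itself into DataPlayer, and ammo for the rifle, shotgun and Lanzacabezas into DataWeapon.
; An invalid game instance only prints an error.
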(event `self.ReceiveActorBeginOverlap`
  (params (OtherActor :type "Actor Object Reference"))
  (bind _asplayer (`self.AsPlayer`))
  (bind _riflecomponent (`/Game/FirstPerson/Blueprints/BP_FirstPersonCharacter.RifleComponent` (`self.AsPlayer`)))
  (bind _escopetacomponent (`/Game/FirstPerson/Blueprints/BP_FirstPersonCharacter.EscopetaComponent` (`self.AsPlayer`)))
  (bind _lanzacabezas (`/Game/FirstPerson/Blueprints/BP_FirstPersonCharacter.LanzaCabezas` (`self.AsPlayer`)))
  (if (== OtherActor (`self.AsPlayer`))
    (if (`KismetSystemLibrary.IsValid` (`self.AsGameInstance`))
      (`/Engine/EditorBlueprintResources/StandardMacros.DoOnce` false
        (:`Completed`
          (set `/Game/Blueprints/Config/BP_MyGameInstance.Data_Player` (make `/Game/Blueprints/Data_Structures/Data_player` (`/Game/FirstPerson/Blueprints/BP_FirstPersonCharacter.HP` _asplayer) (`/Game/FirstPerson/Blueprints/BP_FirstPersonCharacter.Armadura` _asplayer) (`/Game/FirstPerson/Blueprints/BP_FirstPersonCharacter.DashCoolDown` _asplayer) (`/Game/FirstPerson/Blueprints/BP_FirstPersonCharacter.MaxDashCount` _asplayer) (`/Game/FirstPerson/Blueprints/BP_FirstPersonCharacter.bHasRifle` _asplayer) (`/Game/FirstPerson/Blueprints/BP_FirstPersonCharacter.bHasEscopeta` _asplayer) (`/Game/FirstPerson/Blueprints/BP_FirstPersonCharacter.ActiveWeaponSlot` _asplayer) false (`/Game/FirstPerson/Blueprints/BP_FirstPersonCharacter.bHasLanzacabezas` _asplayer) (`Character.JumpMaxCount` _asplayer) (`|ConvertAsset` self)) (`self.AsGameInstance`))
          (set `/Game/Blueprints/Config/BP_MyGameInstance.Data_Weapon` (make `/Game/Blueprints/Data_Structures/Data_Weapon` (`/Game/FirstPerson/Blueprints/LogicaArmas/BP_Weapon_Component_Rifle.CurrentAmmo` _riflecomponent) (`/Game/FirstPerson/Blueprints/LogicaArmas/BP_Weapon_Component_Rifle.ReserveAmmo` _riflecomponent) (`/Game/FirstPerson/Blueprints/LogicaArmas/BP_Weapon_ComponentEscopeta.CurrentAmmo` _escopetacomponent) (`/Game/FirstPerson/Blueprints/LogicaArmas/BP_Weapon_ComponentEscopeta.ReserveAmmo` _escopetacomponent) (`/Game/FirstPerson/Blueprints/LogicaArmas/BP_Weapon_ComponentLanzaCabezas.CurrentAmmo` _lanzacabezas) (`/Game/FirstPerson/Blueprints/LogicaArmas/BP_Weapon_ComponentLanzaCabezas.ReserveAmmo` _lanzacabezas)) (`self.AsGameInstance`))))
      (else
        (`KismetSystemLibrary.PrintString` "El game instance es invalido")))))

(fn `UserConstructionScript`)