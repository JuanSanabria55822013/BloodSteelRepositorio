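; BP_Armadura is an armor pickup actor that restores the player's armature when overlapped.
; On begin overlap with the stored player reference, it checks that armor is not already at MaxArmature.
; If so, it plays the Recoger sound, calls AddArmature on the player with its configured amount, and destroys itself.
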(event `self.ReceiveActorBeginOverlap`
  (params (OtherActor :type "Actor Object Reference"))
  (bind _asplayer (`self.AsPlayer`))
  (if (== OtherActor (`self.AsPlayer`))
    (if (not (== (`/Game/FirstPerson/Blueprints/BP_FirstPersonCharacter.Armadura` _asplayer) (`/Game/FirstPerson/Blueprints/BP_FirstPersonCharacter.MaxArmature` _asplayer)))
      (`GameplayStatics.PlaySound2D` "/Game/Sonidos/Personaje/recoger.recoger" 1.0 1.0 0.0 null null)
      (`/Game/FirstPerson/Blueprints/BP_FirstPersonCharacter.AddArmature` _asplayer (`self.Add Armature`))
      (`self.K2_DestroyActor`))))

(fn `UserConstructionScript`)