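; BP_Salud is a health pickup that floats in place until the player collects it.
; Two timelines move the static mesh's relative location in an endless loop: one plays forward, the other plays in reverse, and each restarts the other.
; On overlap with the stored AsPlayer reference, which these graphs never assign, it heals the player and destroys itself, unless HP already equals MaxHealth.
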(event `self.ReceiveBeginPlay`
  (bind (_direction _z_axis_movement) (`Timeline|Timeline` :!label _label)
    (:`Update`
      (`SceneComponent.K2_SetRelativeLocation` (`self.StaticMesh`) _z_axis_movement false false))
    (:`Finished`
      (bind (_direction_2 _z_axis_movement_2) (`Timeline|Timeline_0` :!via `ReverseFromEnd`)
        (:`Update`
          (`SceneComponent.K2_SetRelativeLocation` (`self.StaticMesh`) _z_axis_movement_2 false false))
        (:`Finished`
          (goto _label :!via `PlayFromStart`))))))

(event `self.ReceiveActorBeginOverlap`
  (params (OtherActor :type "Actor Object Reference"))
  (bind _asplayer (`self.AsPlayer`))
  (if (== OtherActor (`self.AsPlayer`))
    (if (not (== (`/Game/FirstPerson/Blueprints/BP_FirstPersonCharacter.HP` _asplayer) (`/Game/FirstPerson/Blueprints/BP_FirstPersonCharacter.MaxHealth` _asplayer)))
      (`/Game/FirstPerson/Blueprints/BP_FirstPersonCharacter.Heal` _asplayer (`self.Heal`))
      (`self.K2_DestroyActor`))))

(fn `UserConstructionScript`)