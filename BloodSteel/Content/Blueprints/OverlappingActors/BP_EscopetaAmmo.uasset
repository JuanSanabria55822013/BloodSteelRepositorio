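; BP_EscopetaAmmo is an overlap pickup that gives the player shotgun (escopeta) reserve ammo.
; When the overlapping actor matches its AsPlayer reference, it searches the first-person mesh's child components for the BP_Weapon_ComponentEscopeta.
; It adds a fixed amount to that component's ReserveAmmo, capped at a hard-coded maximum.
; The pickup destroys itself once it finds the component, even if the reserve is already full.
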(event `self.ReceiveActorBeginOverlap`
  (params (OtherActor :type "Actor Object Reference"))
  (if (== OtherActor (`self.AsPlayer`))
    (for _array_element (`SceneComponent.GetChildrenComponents` (`/Game/FirstPerson/Blueprints/BP_FirstPersonCharacter.FirstPersonMesh` (`self.AsPlayer`)) false)
      (bind _asbp_weapon_component_escopeta (cast `/Game/FirstPerson/Blueprints/LogicaArmas/BP_Weapon_ComponentEscopeta` _array_element))
      (if (`KismetSystemLibrary.IsValid` _asbp_weapon_component_escopeta)
        (bind _reserveammo (`/Game/FirstPerson/Blueprints/LogicaArmas/BP_Weapon_ComponentEscopeta.ReserveAmmo` _asbp_weapon_component_escopeta))
        (if (== _reserveammo 24)
          (`self.K2_DestroyActor`)
          (else
            (bind _returnvalue (+ _reserveammo 4))
            (if (>= _returnvalue 24)
              (set `/Game/FirstPerson/Blueprints/LogicaArmas/BP_Weapon_ComponentEscopeta.ReserveAmmo` 24 _asbp_weapon_component_escopeta)
              (else
                (set `/Game/FirstPerson/Blueprints/LogicaArmas/BP_Weapon_ComponentEscopeta.ReserveAmmo` _returnvalue _asbp_weapon_component_escopeta)))
            (`self.K2_DestroyActor`)))))))

(fn `UserConstructionScript`)