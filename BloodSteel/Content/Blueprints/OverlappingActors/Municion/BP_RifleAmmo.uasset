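; Rifle ammo pickup that refills the player's reserve ammo when the player overlaps it.
; On overlap with the AsPlayer reference, it checks for a valid RifleComponent and adds a fixed amount to ReserveAmmo, clamped to a hard-coded maximum.
; The pickup then destroys itself, even if the reserve is already full.
; The AsPlayer reference is not assigned in these graphs.
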(event `self.ReceiveActorBeginOverlap`
  (params (OtherActor :type "Actor Object Reference"))
  (bind _riflecomponent (`/Game/FirstPerson/Blueprints/BP_FirstPersonCharacter.RifleComponent` (`self.AsPlayer`)))
  (bind _reserveammo (`/Game/FirstPerson/Blueprints/LogicaArmas/BP_Weapon_Component_Rifle.ReserveAmmo` _riflecomponent))
  (bind _returnvalue (+ _reserveammo 30))
  (if (== OtherActor (`self.AsPlayer`))
    (if (`KismetSystemLibrary.IsValid` _riflecomponent)
      (if (== _reserveammo 100)
        (`self.K2_DestroyActor`)
        (else
          (if (>= _returnvalue 100)
            (set `/Game/FirstPerson/Blueprints/LogicaArmas/BP_Weapon_Component_Rifle.ReserveAmmo` 100 _riflecomponent)
            (else
              (set `/Game/FirstPerson/Blueprints/LogicaArmas/BP_Weapon_Component_Rifle.ReserveAmmo` _returnvalue _riflecomponent)))
          (`self.K2_DestroyActor`))))))

(fn `UserConstructionScript`)