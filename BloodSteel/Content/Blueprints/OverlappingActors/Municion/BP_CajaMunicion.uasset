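; BP_CajaMunicion is an ammo box pickup that fully refills the player's reserve ammo on overlap.
; On begin overlap it compares the other actor to its AsPlayer reference, which is not assigned in this graph.
; If RifleComponent is valid, it sets reserve ammo to maximum on the rifle, Escopeta and LanzaCabezas weapons, then destroys itself.
; The shotgun and LanzaCabezas components get no validity check of their own.
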(event `self.ReceiveActorBeginOverlap`
  (params (OtherActor :type "Actor Object Reference"))
  (bind _asplayer (`self.AsPlayer`))
  (bind _escopetacomponent (`/Game/FirstPerson/Blueprints/BP_FirstPersonCharacter.EscopetaComponent` _asplayer))
  (bind _lanzacabezas (`/Game/FirstPerson/Blueprints/BP_FirstPersonCharacter.LanzaCabezas` _asplayer))
  (bind _riflecomponent (`/Game/FirstPerson/Blueprints/BP_FirstPersonCharacter.RifleComponent` _asplayer))
  (if (== OtherActor (`self.AsPlayer`))
    (if (`KismetSystemLibrary.IsValid` _riflecomponent)
      (set `/Game/FirstPerson/Blueprints/LogicaArmas/BP_Weapon_Component_Rifle.ReserveAmmo` (`/Game/FirstPerson/Blueprints/LogicaArmas/BP_Weapon_Component_Rifle.MaxReserveAmmo` _riflecomponent) _riflecomponent)
      (set `/Game/FirstPerson/Blueprints/LogicaArmas/BP_Weapon_ComponentEscopeta.ReserveAmmo` (`/Game/FirstPerson/Blueprints/LogicaArmas/BP_Weapon_ComponentEscopeta.MaxReseveAmmo` _escopetacomponent) _escopetacomponent)
      (set `/Game/FirstPerson/Blueprints/LogicaArmas/BP_Weapon_ComponentLanzaCabezas.ReserveAmmo` (`/Game/FirstPerson/Blueprints/LogicaArmas/BP_Weapon_ComponentLanzaCabezas.MaxReserveAmmo` _lanzacabezas) _lanzacabezas)
      (`self.K2_DestroyActor`))))

(fn `UserConstructionScript`)