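; BP_Tramp1 is a trap actor that repeatedly changes the player's health or armor while they overlap it.
; On begin overlap with the stored AsPlayer reference, it calls AddHP when Armadura is zero, otherwise AddArmadura, using its HPToAdd and ArmaduraToAdd amounts.
; A one-second Delay loops back to the overlap checks, so the effect ticks until the player leaves.
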(event `self.ReceiveActorBeginOverlap`
  (params (OtherActor :type "Actor Object Reference"))
  (bind _asplayer (`self.AsPlayer`))
  (if (== OtherActor _asplayer) :!label _label
    (if (`self.IsOverlappingActor` _asplayer)
      (if (== (`/Game/FirstPerson/Blueprints/BP_FirstPersonCharacter.Armadura` (`self.AsPlayer`)) 0)
        (`/Game/Blueprints/FunctionLibraries/FL_HPArmadura.AddHP` (`self.HPToAdd`) (`self.AsPlayer`))
        (else
          (`/Game/Blueprints/FunctionLibraries/FL_HPArmadura.AddArmadura` (`self.ArmaduraToAdd`) (`self.AsPlayer`))))
      (`KismetSystemLibrary.Delay` 1.0)
      (goto _label))))

(fn `UserConstructionScript`)