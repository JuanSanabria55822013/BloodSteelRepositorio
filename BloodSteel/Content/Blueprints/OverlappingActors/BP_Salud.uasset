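; BP_Salud is a health pickup actor that restores HP to the player on overlap.
; It reacts only when the overlapping actor matches its AsPlayer reference, which is not assigned in this graph.
; Below or above exactly 100 HP, it passes HPToAdd and the player to AddHP, defined outside these graphs.
; The pickup destroys itself either way, so it is consumed even at 100 HP.
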(event `self.ReceiveActorBeginOverlap`
  (params (OtherActor :type "Actor Object Reference"))
  (if (== OtherActor (`self.AsPlayer`))
    (if (== (`/Game/FirstPerson/Blueprints/BP_FirstPersonCharacter.HP` (`self.AsPlayer`)) 100)
      (`self.K2_DestroyActor`)
      (else
        (`/Game/Blueprints/FunctionLibraries/FL_HPArmadura.AddHP` (`self.HPToAdd`) (`self.AsPlayer`))
        (`self.K2_DestroyActor`)))))

(fn `UserConstructionScript`)