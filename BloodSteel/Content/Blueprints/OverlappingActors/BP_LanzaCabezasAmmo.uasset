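; Ammo pickup for the LanzaCabezas weapon, triggered when the actor stored in AsPlayer overlaps it.
; It searches the direct children of the player's FirstPersonMesh for BP_Weapon_ComponentLanzaCabezas and adds two to its ReserveAmmo, capped at ten.
; Once it finds a valid weapon component the pickup destroys itself, even if the reserve is already full.
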(event `self.ReceiveActorBeginOverlap`
  (params (OtherActor :type "Actor Object Reference"))
  (if (== OtherActor (`self.AsPlayer`))
    (for _array_element (`SceneComponent.GetChildrenComponents` (`/Game/FirstPerson/Blueprints/BP_FirstPersonCharacter.FirstPersonMesh` (`self.AsPlayer`)) false)
      (bind _asbp_weapon_component_lanza_cabezas (cast `/Game/FirstPerson/Blueprints/LogicaArmas/BP_Weapon_ComponentLanzaCabezas` _array_element))
      (if (`KismetSystemLibrary.IsValid` _asbp_weapon_component_lanza_cabezas)
        (bind _reserveammo (`/Game/FirstPerson/Blueprints/LogicaArmas/BP_Weapon_ComponentLanzaCabezas.ReserveAmmo` _asbp_weapon_component_lanza_cabezas))
        (if (== _reserveammo 10)
          (`self.K2_DestroyActor`)
          (else
            (bind _returnvalue (+ _reserveammo 2))
            (if (>= _returnvalue 10)
              (set `/Game/FirstPerson/Blueprints/LogicaArmas/BP_Weapon_ComponentLanzaCabezas.ReserveAmmo` 10 _asbp_weapon_component_lanza_cabezas)
              (else
                (set `/Game/FirstPerson/Blueprints/LogicaArmas/BP_Weapon_ComponentLanzaCabezas.ReserveAmmo` _returnvalue _asbp_weapon_component_lanza_cabezas)))
            (`self.K2_DestroyActor`)))))))

(fn `UserConstructionScript`)