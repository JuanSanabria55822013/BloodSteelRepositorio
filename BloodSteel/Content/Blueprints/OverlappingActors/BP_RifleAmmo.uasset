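; Rifle ammo pickup that adds reserve ammo when the player overlaps it.
; On overlap it searches the child components of the player's first-person mesh for rifle weapon components.
; For a rifle it finds, it adds a fixed amount to reserve ammo, capped at a hardcoded maximum.
; The pickup then destroys itself, even if the reserve was already full.
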(event `self.ReceiveActorBeginOverlap`
  (params (OtherActor :type "Actor Object Reference"))
  (if (== OtherActor (`self.AsPlayer`))
    (for _array_element (`SceneComponent.GetChildrenComponents` (`/Game/FirstPerson/Blueprints/BP_FirstPersonCharacter.FirstPersonMesh` (`self.AsPlayer`)) false)
      (bind _asbp_weapon_component (cast `/Game/FirstPerson/Blueprints/BP_Weapon_Component_Rifle` _array_element))
      (if (`KismetSystemLibrary.IsValid` _asbp_weapon_component)
        (bind _reserveammo (`/Game/FirstPerson/Blueprints/BP_Weapon_Component_Rifle.ReserveAmmo` _asbp_weapon_component))
        (if (== _reserveammo 100)
          (`self.K2_DestroyActor`)
          (else
            (bind _returnvalue (+ _reserveammo 30))
            (if (>= _returnvalue 100)
              (set `/Game/FirstPerson/Blueprints/BP_Weapon_Component_Rifle.ReserveAmmo` 100 _asbp_weapon_component)
              (else
                (set `/Game/FirstPerson/Blueprints/BP_Weapon_Component_Rifle.ReserveAmmo` _returnvalue _asbp_weapon_component)))
            (`self.K2_DestroyActor`)))))))

(fn `UserConstructionScript`)